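; Function library for the card game's chapter mode, resolving card placements and moving each player's hero between placements, the portal and the arena.
; Playing a placement moves the hero there, plays its first card, then sends it to the graveyard.
; Monster cards spawn an AI enemy and start combat; others charge cost and run abilities until one fails.
; Helpers advance placement index, handle cached buffs, set completion flags and notify the game state.
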(fn `Get Hero for Player ID (Server Only)`
  (params (`Player ID` :type Integer))
  (returns (Hero :type "/Game/Crystaline/Blueprints/Hero Object Reference"))
  (return (`/Game/CCGToolkit/Blueprints/Gameplay/BoardPlayer.Hero Character` (`/Game/CCGToolkit/Blueprints/CardGamePlayerController.BoardPlayer_Ref` (cast `/Game/CCGToolkit/Blueprints/CardGamePlayerController` (`/Game/CCGToolkit/Blueprints/FunctionLibraries/Controller_FunctionLibrary.GetControllerReferenceFromID(ServerOnly)` `Player ID`) :!pure true)))))

(fn `Get Placement of Index`
  (params (`Card Placements` :type "Array of /Game/CCGToolkit/Blueprints/Gameplay/CardPlacement Object Reference") (Index :type Integer))
  (returns (Placement :type "/Game/CCGToolkit/Blueprints/Gameplay/CardPlacement Object Reference"))
  (for _array_element `Card Placements`
    (if (== (`/Game/CCGToolkit/Blueprints/Gameplay/CardPlacement.Chapter Index` _array_element) Index)
      (return _array_element)))
  (`KismetSystemLibrary.PrintString` null "Placement Not Found !")
  (return null))

(fn `Get Portal`
  (returns (Portal :type "/Game/Crystaline/Blueprints/Chapter_Portal Object Reference"))
  (bind _outactors (`GameplayStatics.GetAllActorsOfClass` null "/Game/Crystaline/Blueprints/Chapter_Portal.Chapter_Portal_C"))
  (bind _output (`|GetArrayItem` _outactors))
  (`/Engine/EditorBlueprintResources/StandardMacros.IsValid` _output
    (:`Is Valid`
      (return _output))
    (:`Is Not Valid`
      (`KismetSystemLibrary.PrintString` null "Portal not found in Level" true true (struct :`R` 1.0 :`A` 1.0))
      (return null))))

(fn `Get Portal Location`
  (params (`Player ID` :type Integer))
  (returns (ReturnValue :type "Vector Structure"))
  (return (`/Game/Crystaline/Blueprints/Chapter_Portal.Get Player Location` (`self.Get Portal` null) `Player ID`)))

(fn `Go to Portal`
  (params (`Player ID` :type Integer))
  (`AIController.MoveToLocation` (`AIBlueprintHelperLibrary.GetAIController` (`self.Get Hero for Player ID (Server Only)` `Player ID`)) (`self.Get Portal Location` `Player ID`) 0.0 true false false true null true)
  (set `/Game/CCGToolkit/Blueprints/CardGamePlayerState.Finished Chapter` true (cast `/Game/CCGToolkit/Blueprints/CardGamePlayerState` (`/Game/CCGToolkit/Blueprints/FunctionLibraries/Controller_FunctionLibrary.GetControllerPlayerState(ServerOnly)` `Player ID`) :!pure true))
  (`/Game/CCGToolkit/Blueprints/CardGameState.Server_Action Played` (cast `/Game/CCGToolkit/Blueprints/CardGameState` (`GameplayStatics.GetGameState` null) :!pure true) `Player ID` 2.0 true))

(fn `Move to Arena`
  (params (`Player ID` :type Integer))
  (`AIController.MoveToLocation` (`AIBlueprintHelperLibrary.GetAIController` (`self.Get Hero for Player ID (Server Only)` `Player ID`)) (`/Game/Crystaline/Blueprints/Chapter_Portal.Get Player Fight Location` (`self.Get Portal` null) `Player ID`) -1.0 true false false true null true))

(fn `Next Player Placement`
  (params (`Player ID` :type Integer))
  (bind _ascard_game_player_state (`/Game/CCGToolkit/Blueprints/FunctionLibraries/Controller_FunctionLibrary.GetPlayerCardGameState(ServerOnly)` `Player ID`))
  (`/Engine/EditorBlueprintResources/StandardMacros.IncrementInt` (`/Game/CCGToolkit/Blueprints/CardGamePlayerState.Next Placement Index` _ascard_game_player_state)
    (:`  `
      (`/Game/CCGToolkit/Blueprints/CardGamePlayerState.HandleCachedBuffs` _ascard_game_player_state))))

(fn `Play Card Placement`
  (params (`Card placement` :type "/Game/CCGToolkit/Blueprints/Gameplay/CardPlacement Object Reference"))
  (bind _playerindex (`/Game/CCGToolkit/Blueprints/Gameplay/CardPlacement.PlayerIndex` `Card placement`))
  (bind _ascard_game_state (cast `/Game/CCGToolkit/Blueprints/CardGameState` (`GameplayStatics.GetGameState` null) :!pure true))
  (bind _output (`|GetArrayItem` (`/Game/CCGToolkit/Blueprints/Gameplay/CardPlacement.Card_Array` `Card placement`)))
  (`AIController.MoveToLocation` (cast `AIController` (`Pawn.GetController` (`/Game/CCGToolkit/Blueprints/Gameplay/CardPlacement.Get Hero Character` `Card placement`)) :!pure true) (`SceneComponent.K2_GetComponentLocation` (`/Game/CCGToolkit/Blueprints/Gameplay/CardPlacement.Hero Position` `Card placement`)) 0.0 true false false false null true)
  (`/Engine/EditorBlueprintResources/StandardMacros.IsValid` _output
    (:`Is Valid`
      (`self.Play Chapter Card` _output)
      (`/Game/CCGToolkit/Blueprints/Gameplay/3DCard.ForceMoveCardDirectlyToGraveyard` _output (`/Game/CCGToolkit/Blueprints/Gameplay/CardPlacement.Graveyard_Ref` `Card placement`))
      (`/Game/CCGToolkit/Blueprints/Gameplay/CardPlacement.RemoveCardFrom Placement` `Card placement` _output))
    (:`Is Not Valid`
      (`self.Next Player Placement` _playerindex)
      (`/Game/CCGToolkit/Blueprints/CardGameState.Server_Action Played` _ascard_game_state _playerindex 1.0 (not (`/Game/CCGToolkit/Blueprints/CardGameState.Actions Enabled` _ascard_game_state))))))

(fn `Play Chapter Card`
  (params (Card :type "/Game/CCGToolkit/Blueprints/Gameplay/3DCard Object Reference"))
  (bind _owningplayerid (`/Game/CCGToolkit/Blueprints/Gameplay/3DCard.OwningPlayerID` Card))
  (if (`|EnumEquality` (`/Game/CCGToolkit/Blueprints/Gameplay/3DCard.Type` Card) "NewEnumerator0")
    ;[1 1 1] Spawn Monster
    (`self.Spawn Monster` Card)
    (else
      (bind (_valid _cost _error_message) (`/Game/CCGToolkit/Blueprints/FunctionLibraries/Card_FunctionLibrary.ChargeCardCost` _owningplayerid false (`/Game/CCGToolkit/Blueprints/Gameplay/3DCard.CardDataStruct` Card) "NewEnumerator0"))
      (if _valid
        (`self.Run All Abilities` Card)
        (else
          (`/Game/CCGToolkit/Blueprints/CardGamePlayerController.LogNotificationMessage` (cast `/Game/CCGToolkit/Blueprints/CardGamePlayerController` (`/Game/CCGToolkit/Blueprints/FunctionLibraries/Controller_FunctionLibrary.GetControllerReferenceFromID(ServerOnly)` _owningplayerid) :!pure true) _error_message (struct :`R` 1.0 :`A` 1.0))))
      (`self.Next Player Placement` _owningplayerid)
      (`/Game/CCGToolkit/Blueprints/CardGameState.Server_Action Played` (cast `/Game/CCGToolkit/Blueprints/CardGameState` (`GameplayStatics.GetGameState` null) :!pure true) _owningplayerid 1.0 true))))

(fn `Run All Abilities`
  (params (Card :type "/Game/CCGToolkit/Blueprints/Gameplay/3DCard Object Reference"))
  (for (_array_element _array_index) (`/Game/CCGToolkit/Blueprints/Gameplay/3DCard.Ability_Struct_Refs` Card)
    (bind _succesful (`/Game/CCGToolkit/Blueprints/Gameplay/3DCard.RunCardAbility` Card _array_index))
    (if (not _succesful)
      (`KismetSystemLibrary.PrintString` null "Canceling Abilities Effect.")
      (return))))

(fn `Set Player Completed Placement`
  (params (`Player ID` :type Integer) (Completed :type Boolean))
  (set `/Game/CCGToolkit/Blueprints/CardGamePlayerState.Completed Placement` Completed (cast `/Game/CCGToolkit/Blueprints/CardGamePlayerState` (`/Game/CCGToolkit/Blueprints/FunctionLibraries/Controller_FunctionLibrary.GetControllerPlayerState(ServerOnly)` `Player ID`) :!pure true)))

(fn `Spawn Monster`
  (params (`3D Card` :type "/Game/CCGToolkit/Blueprints/Gameplay/3DCard Object Reference"))
  (bind (_aggressive _monsterclass) (break `/Game/CCGToolkit/CardGame/Structs/CardStructs/Monster_Struct` (`.Monster_78_71C7E7A2471D18DC8416C688EC905216` (break `/Game/CCGToolkit/CardGame/Structs/CardStructs/Card_Struct` (`/Game/CCGToolkit/Blueprints/Gameplay/3DCard.CardDataStruct` `3D Card`)))))
  (bind (_returnvalue_location _returnvalue_rotation _returnvalue_scale) (`KismetMathLibrary.BreakTransform` (`SceneComponent.K2_GetComponentToWorld` (`/Game/CCGToolkit/Blueprints/Gameplay/CardPlacement. Monster Spawn Loc` (`/Game/CCGToolkit/Blueprints/Gameplay/3DCard.PlacementOwner` `3D Card`)))))
  (bind _returnvalue (`AIBlueprintHelperLibrary.SpawnAIFromClass` null _monsterclass null _returnvalue_location (`KismetMathLibrary.MakeRotator` 0.0 0.0 (.yaw _returnvalue_rotation))))
  (`Actor.SetActorScale3D` _returnvalue _returnvalue_scale)
  (bind _asmonster_c (cast `/Game/Crystaline/Blueprints/Monster_C` _returnvalue :!pure true))
  (`/Game/Crystaline/Blueprints/Monster_C.Init Stats` _asmonster_c `3D Card`)
  (`/Game/Crystaline/Blueprints/Char.Start Combat` (`/Game/CCGToolkit/Blueprints/Gameplay/CardPlacement.Get Hero Character` (`/Game/CCGToolkit/Blueprints/Gameplay/3DCard.PlacementOwner` `3D Card`)) _asmonster_c _aggressive))