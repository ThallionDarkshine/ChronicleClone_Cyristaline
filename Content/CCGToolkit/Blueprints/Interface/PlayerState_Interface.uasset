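; Blueprint interface for a CCG player state, exposing calls to change a player's combat stats and resources.
; It declares increase and decrease functions for mana, gold, strength and armor, plus health gain and damage to the player.
; It also declares a per-turn mana function and a weapon consume call.
; All functions are empty signatures, so the implementing class supplies the logic.
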(fn `ConsumeWeapon`
  (return))

(fn `Deal Damage to Player`
  (params (Damage :type Integer))
  (returns (ReturnHealth :type Integer))
  (return 0))

(fn `DecreasePlayerArmor`
  (params (Value :type Integer))
  (returns (`New Armor` :type Integer))
  (return 0))

(fn `DecreasePlayerGold`
  (params (Value :type Integer))
  (returns (`New Value` :type Integer))
  (return 0))

(fn `DecreasePlayerMana`
  (params (DecreaseBy :type Integer))
  (returns (ReturnMana :type Integer))
  (return 0))

(fn `DecreasePlayerStrength`
  (params (Value :type Integer))
  (returns (`New Strength` :type Integer))
  (return 0))

(fn `GetManaForTurn`
  (returns (ReturnMana :type Integer))
  (return 0))

(fn `IncreasePlayerArmor`
  (params (Value :type Integer))
  (returns (`New Armor` :type Integer))
  (return 0))

(fn `IncreasePlayerGold`
  (params (Value :type Integer))
  (returns (`New Value` :type Integer))
  (return 0))

(fn `IncreasePlayerHealth`
  (params (IncreaseBy :type Integer))
  (returns (ReturnHealth :type Integer))
  (return 0))

(fn `IncreasePlayerMana`
  (params (IncreaseBy :type Integer))
  (returns (ReturnMana :type Integer))
  (return 0))

(fn `IncreasePlayerStrength`
  (params (Value :type Integer))
  (returns (`New Value` :type Integer))
  (return 0))