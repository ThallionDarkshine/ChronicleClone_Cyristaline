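; Chapter Portal Blueprint that provides world positions for two players at a chapter portal, both a standard location and a fight location.
; Two lookup functions switch on PlayerID (1 or 2) and return the world location of the matching marker component.
; The event graph and construction script hold no logic, so the Blueprint only answers position queries.
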(fn `Get Player Fight Location`
  (params (`Player ID` :type Integer))
  (returns (ReturnValue :type "Vector Structure"))
  (switch `int` `Player ID`
    (:`1`
      (return (`SceneComponent.K2_GetComponentLocation` (`self.Player1 Fight Loc`))))
    (:`2`
      (return (`SceneComponent.K2_GetComponentLocation` (`self.Player2 Fight Loc`))))))

(fn `Get Player Location`
  (params (`Player ID` :type Integer))
  (returns (ReturnValue :type "Vector Structure"))
  (switch `int` `Player ID`
    (:`1`
      (return (`SceneComponent.K2_GetComponentLocation` (`self.Player1 Location`))))
    (:`2`
      (return (`SceneComponent.K2_GetComponentLocation` (`self.Player2 Location`))))))

(fn `UserConstructionScript`)