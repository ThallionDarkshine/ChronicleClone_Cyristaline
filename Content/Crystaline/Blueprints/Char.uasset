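; Base combat character for a turn-based card game, with a health indicator widget and server/client-named events for attack, hit and death.
; StartCombat links both fighters, then after a delay triggers either a death or one attack, with MonsterAggresive choosing the attacker.
; Attacks play a montage and apply Attack-based damage.
; Death calls an empty LootReward, freezes and expires the body, and advances the turn if the enemy is a Hero.
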(event `self.ReceiveBeginPlay`
  (bind _ashealth_indicator (cast `/Game/Crystaline/Blueprints/Wdigets/Health_Indicator` (`WidgetComponent.GetUserWidgetObject` (`self.Health Indicator`))))
  (set `/Game/Crystaline/Blueprints/Wdigets/Health_Indicator.Char` self _ashealth_indicator))

(event `self.ReceiveTick`
  (params (DeltaSeconds :type "Float (single-precision)"))
  (`/Engine/EditorBlueprintResources/ActorMacros.Switch Has Authority`
    (:`Authority`
      (set `self.Movement Speed` (`KismetMathLibrary.VSize` (`self.GetVelocity`))))))

(event `Start Combat`
  (params (Enemy :type "/Game/Crystaline/Blueprints/Char Object Reference") (`Monster Aggresive` :type Boolean))
  (set `self.Enemy` Enemy)
  (set `/Game/Crystaline/Blueprints/Char.Enemy` self Enemy)
  (`KismetSystemLibrary.Delay` 1.0)
  (if (== (`self.Health`) 0)
    (`self.Server Death`)
    (elif (== (`/Game/Crystaline/Blueprints/Char.Health` Enemy) 0)
      (`self.Server Death` Enemy)
      (elif `Monster Aggresive`
        (`self.Server Attack` Enemy self)
        (else
          (`self.Server Attack` Enemy))))))

(event `Server Attack`
  (params (Enemy :type "/Game/Crystaline/Blueprints/Char Object Reference"))
  (`self.Client Attack`)
  (`KismetSystemLibrary.Delay` 0.5)
  (`GameplayStatics.ApplyDamage` Enemy (`KismetMathLibrary.Conv_IntToDouble` (`self.Get Attack Power`)) null self))

(event `Client Attack`
  (`|PlayMontage` (`self.Mesh`) "/Game/Crystaline/Anim/Attack_Montage.Attack_Montage"))

(event `Client Hit`
  (`|PlayMontage` (`self.Mesh`) "/Game/Crystaline/Anim/Hit_Montage.Hit_Montage"))

(event `Server Death`
  (`self.Client Death`)
  (`self.Loot Reward`)
  (bind _ashero (cast `/Game/Crystaline/Blueprints/Hero` (`self.Enemy`)))
  (bind _cardgameplayerid (`/Game/CCGToolkit/Blueprints/CardGamePlayerState.CardGamePlayerId` (`/Game/Crystaline/Blueprints/Hero.Player State Ref` _ashero)))
  (`/Game/CCGToolkit/Blueprints/FunctionLibraries/Chapter_FunctionLibrary.Set Player Completed Placement` _cardgameplayerid true)
  (`/Game/CCGToolkit/Blueprints/FunctionLibraries/Chapter_FunctionLibrary.Next Player Placement` _cardgameplayerid)
  (`/Game/CCGToolkit/Blueprints/CardGameState.Server_Action Played` (cast `/Game/CCGToolkit/Blueprints/CardGameState` (`GameplayStatics.GetGameState`) :!pure true) _cardgameplayerid 1.0 true))

(event `Client Death`
  (bind _mesh (`self.Mesh`))
  (`PrimitiveComponent.SetCollisionResponseToChannel` (`self.CapsuleComponent`) "ECC_Pawn" "ECR_Ignore")
  (`|PlayMontage` _mesh "/Game/Crystaline/Anim/Death_Montage.Death_Montage"
    (:`then`
      (`KismetSystemLibrary.Delay` 0.75)
      (set `SkeletalMeshComponent.bPauseAnims` true _mesh)
      (`self.SetLifeSpan` 1.0))))

(fn `Get Attack Power`
  (returns (Attack :type Integer))
  (return (`self.Attack`)))

(fn `Loot Reward`)

(fn `UserConstructionScript`)