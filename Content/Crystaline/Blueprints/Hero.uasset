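; Hero actor for a card game, fighting monsters and a final battle using stats from the player state.
; Incoming damage is passed to the player state, leading to death at zero or a hit reaction.
; After a delay it counterattacks aggressive monsters and non-monster final-battle foes, while non-aggressive monsters hand the action back to CardGameState.
; Attacks apply the player state's attack damage after a client-side attack cue, then consume the weapon.
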(event `self.ReceiveAnyDamage`
  (params (Damage :type "Float (single-precision)") (DamageType :type "DamageType Object Reference") (InstigatedBy :type "Controller Object Reference") (DamageCauser :type "Actor Object Reference"))
  (bind (_asmonster_c _bsuccess) (cast `/Game/Crystaline/Blueprints/Monster_C` DamageCauser :!pure true))
  (bind _enemy (`self.Enemy`))
  (bind _ascard_game_state (cast `/Game/CCGToolkit/Blueprints/CardGameState` (`GameplayStatics.GetGameState`) :!pure true))
  (bind _cardgameplayerid (`/Game/CCGToolkit/Blueprints/CardGamePlayerState.CardGamePlayerId` (`self.Player State Ref`)))
  (bind _returnhealth (message `/Game/CCGToolkit/Blueprints/Interface/PlayerState_Interface.Deal Damage to Player` (`self.Player State Ref`) (`KismetMathLibrary.FTrunc` Damage)))
  (if (== _returnhealth 0)
    (`self.Server Death`)
    (else
      (`self.Client Hit`)
      (`KismetSystemLibrary.Delay` 0.5)
      (if _bsuccess
        (if (`/Game/Crystaline/Blueprints/Monster_C.Aggressive` _asmonster_c)
          (`self.Server Attack` _enemy)
          (else
            (`/Game/CCGToolkit/Blueprints/FunctionLibraries/Chapter_FunctionLibrary.Set Player Completed Placement` _cardgameplayerid)
            (`/Game/CCGToolkit/Blueprints/CardGameState.Server_Action Played` _ascard_game_state _cardgameplayerid 0.15 (`/Game/CCGToolkit/Blueprints/CardGameState.Actions Enabled` _ascard_game_state))))
        (else
          ;[1 1 1] Final Battle
          (`self.Server Attack` _enemy))))))

(event `self.Server Attack`
  (params (Enemy :type "/Game/Crystaline/Blueprints/Char Object Reference"))
  (if (> (`/Game/CCGToolkit/Blueprints/CardGamePlayerState.Health` (`self.Player State Ref`)) 0)
    (`self.Client Attack`)
    (`KismetSystemLibrary.Delay` 0.5)
    (`GameplayStatics.ApplyDamage` Enemy (`KismetMathLibrary.Conv_IntToDouble` (`self.Get Attack Power`)) null self)
    (`/Game/CCGToolkit/Blueprints/CardGamePlayerState.ConsumeWeapon` (`self.Player State Ref`))))

(event `Continue Combat`
  (bind _enemy (`self.Enemy`))
  (bind _asmonster_c (cast `/Game/Crystaline/Blueprints/Monster_C` _enemy))
  (`self.Start Combat` _enemy (`/Game/Crystaline/Blueprints/Monster_C.Aggressive` _asmonster_c)))

(fn `Get Attack Power`
  (returns (Attack :type Integer))
  (return (`/Game/CCGToolkit/Blueprints/CardGamePlayerState.Get Attack Damage` (`self.Player State Ref`))))

(fn `Update Hero`
  (params (`Player State` :type "/Game/CCGToolkit/Blueprints/CardGamePlayerState Object Reference"))
  (set `self.Attack` (`/Game/CCGToolkit/Blueprints/CardGamePlayerState.Strength` `Player State`))
  (set `self.Health` (`/Game/CCGToolkit/Blueprints/CardGamePlayerState.Health` `Player State`)))

(fn `UserConstructionScript`
  (`parent.UserConstructionScript`))