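; Monster character for the card game, initialized on the server with health, attack and aggression from its 3D card.
; Damage lowers health and shows a stat widget; zero health triggers ServerDeath, otherwise it plays a hit.
; Surviving non-aggressive monsters attack the damaging Hero back, while aggressive ones reopen that player's placement and report the action played.
; LootReward grants the placement owner the card's gold and runs its abilities.
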(event `self.Loot Reward`
  (bind (_carddatastruct_name _carddatastruct_class _carddatastruct_type _carddatastruct_subtype _carddatastruct_rarity _carddatastruct_special _carddatastruct_visual _carddatastruct_attack _carddatastruct_health _carddatastruct_gold) (break `/Game/CCGToolkit/CardGame/Structs/CardStructs/Card_Struct` (`/Game/CCGToolkit/Blueprints/Gameplay/3DCard.CardDataStruct` (`self.3D Card`))))
  (`/Engine/EditorBlueprintResources/ActorMacros.Switch Has Authority`
    (:`Authority`
      (`/Game/CCGToolkit/Blueprints/CardGamePlayerState.IncreasePlayerGold` (cast `/Game/CCGToolkit/Blueprints/CardGamePlayerState` (`Controller.PlayerState` (`/Game/CCGToolkit/Blueprints/Gameplay/CardPlacement.Get Placement Controller` (`/Game/CCGToolkit/Blueprints/Gameplay/3DCard.PlacementOwner` (`self.3D Card`)))) :!pure true) _carddatastruct_gold)
      (`/Game/CCGToolkit/Blueprints/FunctionLibraries/Chapter_FunctionLibrary.Run All Abilities` (`self.3D Card`)))))

(event `self.ReceiveAnyDamage`
  (params (Damage :type "Float (single-precision)") (DamageType :type "DamageType Object Reference") (InstigatedBy :type "Controller Object Reference") (DamageCauser :type "Actor Object Reference"))
  (bind _returnvalue (`KismetMathLibrary.FTrunc` Damage))
  (bind _ashero (cast `/Game/Crystaline/Blueprints/Hero` DamageCauser :!pure true))
  (bind _ascard_game_state (cast `/Game/CCGToolkit/Blueprints/CardGameState` (`GameplayStatics.GetGameState`) :!pure true))
  (bind _cardgameplayerid (`/Game/CCGToolkit/Blueprints/CardGamePlayerState.CardGamePlayerId` (`/Game/Crystaline/Blueprints/Hero.Player State Ref` _ashero)))
  ;[1 1 1] On Damage Recieved
  (bind _output_get (set `self.Health` (`KismetMathLibrary.Max` (- (`self.Health`) _returnvalue))))
  (`/Game/CCGToolkit/Blueprints/CardGamePlayerState.Client Register Stat Update Widget` (cast `/Game/CCGToolkit/Blueprints/CardGamePlayerState` (`/Game/CCGToolkit/Blueprints/FunctionLibraries/Controller_FunctionLibrary.GetControllerPlayerState(ServerOnly)` (`/Game/CCGToolkit/Blueprints/Gameplay/3DCard.OwningPlayerID` (`self.3D Card`))) :!pure true) "NewEnumerator0" _returnvalue false self)
  (if (== _output_get 0)
    (`self.Server Death`)
    (else
      (`self.Client Hit`)
      (`KismetSystemLibrary.Delay` 0.5)
      (if (`self.Aggressive`)
        (`/Game/CCGToolkit/Blueprints/FunctionLibraries/Chapter_FunctionLibrary.Set Player Completed Placement` _cardgameplayerid)
        (`/Game/CCGToolkit/Blueprints/CardGameState.Server_Action Played` _ascard_game_state _cardgameplayerid 0.15 (`/Game/CCGToolkit/Blueprints/CardGameState.Actions Enabled` _ascard_game_state))
        (else
          (`self.Server Attack` _ashero))))))

(fn `Init Stats`
  (params (`3D Card` :type "/Game/CCGToolkit/Blueprints/Gameplay/3DCard Object Reference"))
  (bind _3d_card (`self.3D Card`))
  (`/Engine/EditorBlueprintResources/ActorMacros.Switch Has Authority`
    (:`Authority`
      (set `self.3D Card` `3D Card`)
      (set `self.Health` (`/Game/CCGToolkit/Blueprints/Gameplay/3DCard.Health` _3d_card))
      (set `self.Attack` (`/Game/CCGToolkit/Blueprints/Gameplay/3DCard.Attack` _3d_card))
      (set `self.Aggressive` (`.Aggressive_1_3A8A572A4E32114C512D2F8688B8C1D9` (break `/Game/CCGToolkit/CardGame/Structs/CardStructs/Monster_Struct` (`.Monster_78_71C7E7A2471D18DC8416C688EC905216` (break `/Game/CCGToolkit/CardGame/Structs/CardStructs/Card_Struct` (`/Game/CCGToolkit/Blueprints/Gameplay/3DCard.CardDataStruct` `3D Card`)))))))))

(fn `UserConstructionScript`)